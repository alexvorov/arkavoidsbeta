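; BP_Cube_1lives is a destructible cube that loses a life when hit by BP_MyBall and may drop a bonus when destroyed.
; Each ball hit decrements Lives, and the cube destroys itself when none remain.
; At BeginPlay a coin flip decides whether SpawnBonus binds to OnDestroyed; a second flip then decides whether BP_Bonus spawns at the cube's location.
; A BP_Bonus1 spawn node is left unconnected and never runs.
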(event Custom|BallIsHit
  (bind _result (Math|Integer|DecrementInt (Variables|Default|GetLives))
    (:%20%20
      (if (<= _result 0)
        (Actor|DestroyActor)))))

(event Custom|SpawnBonus
  (params (DestroyedActor :type Actor%20Object%20Reference))
  (if (== (Math|Random|RandomIntegerinRange 0 1) 0)
    (Game|SpawnActorfromClass "/Game/MyGame/Blueprints/Bonuses/BP_Bonus.BP_Bonus_C" (Math|Transform|MakeTransform (Transformation|GetActorLocation) "-40.000000, 0, 0") "Undefined" 0 0)))

(event Collision|EventActorBeginOverlap
  (params (OtherActor :type Actor%20Object%20Reference)))

(event EventTick
  (params (DeltaSeconds :type Float%20%28single-precision%29)))

(event Collision|EventHit
  (params (MyComp :type Primitive%20Component%20Object%20Reference) (Other :type Actor%20Object%20Reference) (OtherComp :type Primitive%20Component%20Object%20Reference) (bSelfMoved :type Boolean) (HitLocation :type Vector :default "0, 0, 0") (HitNormal :type Vector :default "0, 0, 0") (NormalImpulse :type Vector :default "0, 0, 0") (Hit :type Hit%20Result%20Structure%20%28by%20ref%29))
  (Utilities|Casting|CastToBP_MyBall Other)
  (CallFunction|BallIsHit))

(event EventBeginPlay
  (if (== (Math|Random|RandomIntegerinRange 1 2) 2)
    (EventDispatchers|BindEventtoOnDestroyed (delegate Custom|SpawnBonus))))

(fn ConstructionScript)