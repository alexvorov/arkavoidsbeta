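; Player pawn that launches balls, tracks lives and collects bonuses with its Cube.
; SpawnBall keeps one tracked ball alive while lives remain; its destruction costs a life and fires LivesZero when none are left.
; Cube overlaps with BP_Bonus widen or narrow it, add a life, or spawn a smaller untracked ball.
; Both resizes share a retriggerable delay that restores the default scale.
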(event OnComponentBeginOverlap(Cube)
  (params (OverlappedComponent :type Primitive%20Component%20Object%20Reference) (OtherActor :type Actor%20Object%20Reference) (OtherComp :type Primitive%20Component%20Object%20Reference) (OtherBodyIndex :type Integer) (bFromSweep :type Boolean) (SweepResult :type Hit%20Result%20Structure%20%28by%20ref%29))
  (bind _asbp_bonus (Utilities|Casting|CastToBP_Bonus OtherActor))
  (switch Utilities|FlowControl|Switch|SwitchonE_BonusType (Variables|/Game/MyGame/Blueprints/Bonuses/BP_Bonus.BP_Bonus_C|GetBonusType _asbp_bonus)
    (:NewEnumerator0
      (CallFunction|MaximizeEvent))
    (:NewEnumerator1
      (CallFunction|LifeEvent))
    (:NewEnumerator2
      (CallFunction|BallEvent))
    (:NewEnumerator3
      (CallFunction|MinimizeEvent)))
  (Actor|DestroyActor _asbp_bonus))

(event Custom|SpawnBall
  (if (not (<= (Variables|Default|GetPlayerLives) 0))
    (Variables|Default|GetAliveBall
      (:then)
      (:else
        (bind _returnvalue (Game|SpawnActorfromClass "/Game/MyGame/Blueprints/BP_MyBall.BP_MyBall_C" (Math|Transform|MakeTransform (Transformation|GetWorldLocation (Variables|Default|GetArrow)) "0, 0, 0" "0.750000,0.750000,0.750000") "Undefined" 0 0))
        (bind _output_get (Variables|Default|SetAliveBall _returnvalue))
        (Game|BindEventtoOnDestroyed _output_get (delegate Custom|BallIsDead))))))

(event Custom|BallIsDead
  (params (DestroyedActor :type Actor%20Object%20Reference))
  (bind _result (Math|Integer|DecrementInt (Variables|Default|GetPlayerLives))
    (:%20%20
      (if (<= _result 0)
        (Default|CallLivesZero)))))

(event Custom|MaximizeEvent
  (bind _cube (Variables|Default|GetCube))
  (bind _relativescale3d (Variables|/Script/Engine.SceneComponent|GetRelativeScale3D _cube))
  (Transformation|SetRelativeScale3D _cube (Math|Vector|MakeVector (.x _relativescale3d) (* (.y _relativescale3d) 1.5) (.z _relativescale3d)))
  (CallFunction|MinEvent))

(event Custom|LifeEvent
  (bind _result (Math|Integer|IncrementInt (Variables|Default|GetPlayerLives))
    (:%20%20
      (Default|CallLivesChanged _result))))

(event Custom|BallEvent
  (Game|SpawnActorfromClass "/Game/MyGame/Blueprints/BP_MyBall.BP_MyBall_C" (Math|Transform|MakeTransform (Transformation|GetWorldLocation (Variables|Default|GetArrow)) "0, 0, 0" "0.500000,0.500000,0.500000") "Undefined" 0 0))

(event Custom|MinEvent
  (Utilities|FlowControl|RetriggerableDelay 3.0)
  (Transformation|SetRelativeScale3D (Variables|Default|GetCube) (Variables|Default|GetDefaultScale)))

(event Custom|MinimizeEvent
  (bind _cube (Variables|Default|GetCube))
  (bind _relativescale3d (Variables|/Script/Engine.SceneComponent|GetRelativeScale3D _cube))
  (Transformation|SetRelativeScale3D _cube (Math|Vector|MakeVector (.x _relativescale3d) (* (.y _relativescale3d) 0.66) (.z _relativescale3d)))
  (CallFunction|MinEvent))

(event Collision|EventActorBeginOverlap
  (params (OtherActor :type Actor%20Object%20Reference)))

(event EventTick
  (params (DeltaSeconds :type Float%20%28single-precision%29)))

(event EventBeginPlay
  (Variables|Default|SetDefaultScale (Variables|/Script/Engine.SceneComponent|GetRelativeScale3D (Variables|Default|GetCube))))

(fn ConstructionScript)