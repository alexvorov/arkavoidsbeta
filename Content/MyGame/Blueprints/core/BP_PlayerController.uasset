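; Player controller that drives BP_MyPawn and manages the gameplay HUD and loss screen.
; On possess it binds GameFinished to the pawn's lives-zero event, which swaps the stored HUD for WBP_Loss and switches to UI-only input with a cursor.
; Left_Right input offsets the pawn along Y, scaled by speed and delta time.
; SpawnBall calls the pawn's spawn and also adds another, unstored HUD widget on each press.
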(event Custom|GameFinished
  (Widget|SetVisibility (Variables|Default|GetHUD) "Collapsed")
  (bind _returnvalue (UserInterface|CreateWidget "/Game/MyGame/UI/WBP_Loss.WBP_Loss_C" self))
  (UserInterface|Viewport|AddtoViewport _returnvalue 0)
  (Input|SetInputModeUIOnly self 0 "LockOnCapture")
  (Variables|Default|SetbShowMouseCursor true))

(event EventTick
  (params (DeltaSeconds :type Float%20%28single-precision%29)))

(event EventPossess
  (params (PossessedPawn :type Pawn%20Object%20Reference))
  (bind _asbp_my_pawn (Utilities|Casting|CastToBP_MyPawn PossessedPawn))
  (bind _output_get (Variables|Default|SetMy_Pawn _asbp_my_pawn))
  (EventDispatchers|BindEventtoLivesZero _output_get (delegate Custom|GameFinished)))

(event EventBeginPlay
  (Input|SetInputModeGameOnly self)
  (bind _returnvalue (UserInterface|CreateWidget "/Game/MyGame/UI/WBP_HUD.WBP_HUD_C" self))
  (UserInterface|Viewport|AddtoViewport _returnvalue 0)
  (Variables|Default|SetHUD _returnvalue))

(event Input|ActionEvents|InputActionSpawnBall
  (params (Key :type Key%20Structure))
  (:Pressed
    (Default|SpawnBall (Variables|Default|GetMy_Pawn))
    (bind _returnvalue (UserInterface|CreateWidget "/Game/MyGame/UI/WBP_HUD.WBP_HUD_C"))
    (UserInterface|Viewport|AddtoViewport _returnvalue 0)))

(event Input|AxisEvents|InputAxisLeft_Right
  (params (AxisValue :type Float%20%28single-precision%29))
  (Transformation|AddActorWorldOffset (Variables|Default|GetMy_Pawn) (Math|Vector|MakeVector 0.0 (* AxisValue (Utilities|Time|GetWorldDeltaSeconds) (Variables|Default|GetSpeed)) 0.0)))

(fn ConstructionScript)