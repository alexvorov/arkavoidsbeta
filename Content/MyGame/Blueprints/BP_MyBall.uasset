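; BP_MyBall is a bouncing ball that responds to bonus pickups.
; Tick moves it with a swept offset, reflecting its direction and adding capped speed on blocking hits; Hit plays a sound.
; Overlapping a BP_Bonus1 triggers a size or speed change by BonusType, then calls DestroyActor on itself.
; Size changes (Small shrinks only Y) revert through a retriggerable delay, while speed changes have no timer.
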(event OnComponentBeginOverlap(Sphere)
  (params (OverlappedComponent :type Primitive%20Component%20Object%20Reference) (OtherActor :type Actor%20Object%20Reference) (OtherComp :type Primitive%20Component%20Object%20Reference) (OtherBodyIndex :type Integer) (bFromSweep :type Boolean) (SweepResult :type Hit%20Result%20Structure%20%28by%20ref%29))
  (bind _asbp_bonus_1 (Utilities|Casting|CastToBP_Bonus1 OtherActor))
  (switch Utilities|FlowControl|Switch|SwitchonE_BonusType2 (Variables|/Game/MyGame/Blueprints/Bonuses/BP_Bonus1.BP_Bonus1_C|GetBonusType _asbp_bonus_1)
    (:NewEnumerator0
      (CallFunction|BigBall))
    (:NewEnumerator1
      (CallFunction|SmallBall))
    (:NewEnumerator2
      (CallFunction|SpeedUp))
    (:NewEnumerator3
      (CallFunction|SpeedDown)))
  (Actor|DestroyActor))

(event Custom|BigBall
  (bind _sphere (Variables|Default|GetSphere))
  (bind _relativescale3d (Variables|/Script/Engine.SceneComponent|GetRelativeScale3D _sphere))
  (Transformation|SetRelativeScale3D _sphere (Math|Vector|MakeVector (* (.x _relativescale3d) 1.5) (* (.y _relativescale3d) 1.5) (.z _relativescale3d)))
  (CallFunction|MinEvent))

(event Custom|SmallBall
  (bind _sphere (Variables|Default|GetSphere))
  (bind _relativescale3d (Variables|/Script/Engine.SceneComponent|GetRelativeScale3D _sphere))
  (Transformation|SetRelativeScale3D _sphere (Math|Vector|MakeVector (.x _relativescale3d) (* (.y _relativescale3d) 0.66) (.z _relativescale3d)))
  (CallFunction|MinEvent))

(event Custom|SpeedDown
  (Variables|Default|SetSpeed (/ (Variables|Default|GetSpeed) 1.5)))

(event Custom|MinEvent
  (Utilities|FlowControl|RetriggerableDelay 3.0)
  (Transformation|SetRelativeScale3D (Variables|Default|GetSphere) (Variables|Default|GetDefault%20Scale)))

(event Custom|SpeedUp
  (Variables|Default|SetSpeed (* (Variables|Default|GetSpeed) 1.5)))

(event EventBeginPlay)

(event Collision|EventActorBeginOverlap
  (params (OtherActor :type Actor%20Object%20Reference)))

(event EventTick
  (params (DeltaSeconds :type Float%20%28single-precision%29))
  (bind _sweephitresult (Transformation|AddActorWorldOffset (Math|Vector|MakeVector (.x (* (Variables|Default|GetDirection) (* DeltaSeconds (Variables|Default|GetSpeed)))) (.y (* (Variables|Default|GetDirection) (* DeltaSeconds (Variables|Default|GetSpeed)))) 0.0) true))
  (if (.bBlockingHit (Collision|BreakHitResult _sweephitresult))
    (Variables|Default|SetDirection (Math|Vector|GetReflectionVector (Variables|Default|GetDirection) (.Normal (Collision|BreakHitResult _sweephitresult))))
    (Variables|Default|SetSpeed (Math|Float|Min(Float) (+ (Variables|Default|GetSpeed) (Variables|Default|GetAdded_Speed)) 2e+03))))

(event Collision|EventHit
  (params (MyComp :type Primitive%20Component%20Object%20Reference) (Other :type Actor%20Object%20Reference) (OtherComp :type Primitive%20Component%20Object%20Reference) (bSelfMoved :type Boolean) (HitLocation :type Vector :default "0, 0, 0") (HitNormal :type Vector :default "0, 0, 0") (NormalImpulse :type Vector :default "0, 0, 0") (Hit :type Hit%20Result%20Structure%20%28by%20ref%29))
  (Audio|PlaySound2D "/Game/MyGame/Assets/udar-po-metallicheskomu-predmetu.udar-po-metallicheskomu-predmetu" 1.0 1.0 0.0 0 0))

(fn ConstructionScript)