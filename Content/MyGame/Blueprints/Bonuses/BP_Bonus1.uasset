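; BP_Bonus1 is a moving bonus actor that carries one of four random bonus types and displays it as text.
; The Construction Script randomly picks the BonusType enum value and writes its name to the TextRender component.
; Tick moves the actor with a swept, frame-rate-independent world offset from Direction and Speed, applying only the X component.
; It contains no overlap or pickup logic.
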(event EventBeginPlay)

(event Collision|EventActorBeginOverlap
  (params (OtherActor :type Actor%20Object%20Reference)))

(event EventTick
  (params (DeltaSeconds :type Float%20%28single-precision%29))
  (Transformation|AddActorWorldOffset (Math|Vector|MakeVector (.x (* (Variables|Default|GetDirection) (* DeltaSeconds (Variables|Default|GetSpeed)))) 0.0 0.0) true))

(fn ConstructionScript
  (Variables|Default|SetBonusType (Utilities|Select :Index (Math|Random|RandomIntegerinRange 0 3) :Option%200 "NewEnumerator0" :Option%201 "NewEnumerator1" :Option%202 "NewEnumerator2" :Option%203 "NewEnumerator3"))
  (Rendering|Components|TextRender|SetText (Variables|Default|GetTextRender) (Utilities|Text|ToText(String) (Utilities|String|EnumtoString (Variables|Default|GetBonusType)))))